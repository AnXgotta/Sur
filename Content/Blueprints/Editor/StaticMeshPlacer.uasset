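; Editor placer actor that scatters static mesh components over surfaces within a box area when its construction script runs.
; It line-traces along Z from seeded random XY points, adding a mesh with a shared material at each hit.
; A random MultiGate optionally picks among six meshes, independent of the seed.
; CombineTransformations supplies rotation and scale from base values and seeded variation, while location adds a fixed offset to the hit.
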(fn ConstructionScript
  (bind _returnvalue (Transformation|GetActorLocation))
  (bind _tracedepth (Variables|Default|GetTraceDepth))
  (bind _uniformscalevariation (Variables|Default|GetUniformScaleVariation))
  (bind _transformseed (Variables|Default|GetTransformSeed))
  (bind _boxrange (Variables|Default|GetBoxRange))
  (bind _transformvariation (Variables|Default|GetTransformVariation))
  (bind _transform (Variables|Default|GetTransform))
  (bind _transformseed_2 (Variables|Default|GetTransformSeed))
  (bind _transform_2 (Variables|Default|GetTransform))
  (bind _transformseed_3 (Variables|Default|GetTransformSeed))
  (bind _transformvariation_2 (Variables|Default|GetTransformVariation))
  (bind _radiusbounds (Variables|Default|GetRadiusBounds))
  (bind _radiusbounds_2 (Variables|Default|GetRadiusBounds))
  (bind _scale (Math|Transform|BreakTransform _transformvariation))
  (bind _rotation (Math|Transform|BreakTransform _transform_2))
  (bind _scale_2 (Math|Transform|BreakTransform _transform))
  (bind _rotation_2 (Math|Transform|BreakTransform _transformvariation_2))
  (bind _returnvalue_2 (/ _tracedepth 2.0))
  (bind (_x _y _z) (Math|Vector|BreakVector _returnvalue))
  (bind (_x_2 _y_2) (Math|Vector|BreakVector _radiusbounds))
  (bind (_x_3 _y_3) (Math|Vector|BreakVector _radiusbounds_2))
  (bind (_pitch _yaw _roll) (Class|KismetMathLibrary|BreakRot _rotation))
  (bind (_x_4 _y_4 _z_2) (Math|Vector|BreakVector _scale_2))
  (bind (_pitch_2 _yaw_2 _roll_2) (Class|KismetMathLibrary|BreakRot _rotation_2))
  (bind (_x_5 _y_5 _z_3) (Math|Vector|BreakVector _scale))
  (bind (_x_out _y_out _z_out) (Utilities|CombineTransformations _x_5 _y_5 _z_3 _uniformscalevariation _transformseed_2 _x_4 _y_4 _z_2))
  (bind (_x_out_2 _y_out_2 _z_out_2) (Utilities|CombineTransformations _pitch_2 _yaw_2 _roll_2 1.0 _transformseed _pitch _yaw _roll))
  (Components|Box|SetBoxExtent _boxrange (Math|Vector|MakeVector _x_2 _y_2 (Math|Float|Absolute(Float) _returnvalue_2)) false)
  (Transformation|AddLocalOffset _boxrange (Math|Vector|MakeVector 0.0 0.0 _returnvalue_2) false)
  (Math|Random|SetRandomStreamSeed (Variables|Default|GetTransformSeed) (Variables|Default|GetSeededTransformation))
  (for _index (range 1 (Variables|Default|GetNumberOfMeshes))
    (Variables|Default|SetLocationToAddMesh (Math|Vector|MakeVector (+ (Math|Random|RandomFloatinRangefromStream (* _x_3 -1.0) _x_3 _transformseed_3) _x) (+ (Math|Random|RandomFloatinRangefromStream (* _y_3 -1.0) _y_3 _transformseed_3) _y) _z))
    (bind _outhit (Collision|LineTraceForObjects (Variables|Default|GetLocationToAddMesh) (+ (Variables|Default|GetLocationToAddMesh) (Math|Vector|MakeVector 0.0 0.0 (Variables|Default|GetTraceDepth))) (Variables|Default|GetCollideWith) false 0 "None"))
    (if (!= (.HitActor (Collision|BreakHitResult _outhit)) 0)
      (bind _returnvalue_3 (AddComponent|AddStaticMeshComponent false))
      (if (Variables|AdditionalMeshes|GetUseRandomMeshes)
        (Utilities|FlowControl|MultiGate true true -1
          (:Out%200
            (Components|StaticMesh|SetStaticMesh _returnvalue_3 (Variables|Default|GetStaticMesh)))
          (:Out%201
            (Components|StaticMesh|SetStaticMesh _returnvalue_3 (Variables|AdditionalMeshes|GetRandomStaticMesh1)))
          (:Out%202
            (Components|StaticMesh|SetStaticMesh _returnvalue_3 (Variables|AdditionalMeshes|GetRandomStaticMesh2)))
          (:Out%203
            (Components|StaticMesh|SetStaticMesh _returnvalue_3 (Variables|AdditionalMeshes|GetRandomStaticMesh3)))
          (:Out%204
            (Components|StaticMesh|SetStaticMesh _returnvalue_3 (Variables|AdditionalMeshes|GetRandomStaticMesh4)))
          (:Out%205
            (Components|StaticMesh|SetStaticMesh _returnvalue_3 (Variables|AdditionalMeshes|GetRandomStaticMesh5))))
        (else
          (Components|StaticMesh|SetStaticMesh _returnvalue_3 (Variables|Default|GetStaticMesh))))
      (Rendering|Material|SetMaterial _returnvalue_3 0 (Variables|Default|GetMaterial))
      (Transformation|SetWorldLocation _returnvalue_3 (+ (.Location (Collision|BreakHitResult _outhit)) (.Location (Math|Transform|BreakTransform (Variables|Default|GetTransform)))) false)
      (Transformation|SetRelativeRotation _returnvalue_3 (Class|KismetMathLibrary|MakeRot _x_out_2 _y_out_2 _z_out_2) false)
      (Transformation|SetRelativeScale3D _returnvalue_3 (Math|Vector|MakeVector _x_out _y_out _z_out)))))