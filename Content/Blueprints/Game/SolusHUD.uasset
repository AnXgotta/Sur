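; SolusHUD is the player HUD Blueprint, drawing a screen fade and a centered crosshair.
; Each DrawHUD derives a clamped scale from screen width, draws a black rect using the FadeIn timeline's alpha, and shows the crosshair material only while SolusPlayerController allows input.
; The timeline plays forward on BeginPlay or HudFadeIn and reverses for HudFadeOut or player death, the latter at its own play rate.
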(event Custom|HudFadeIn
  ;[1 0.2974 0.5828] Actual HUD
  (Components|Timeline|SetPlayRate (Variables|Default|GetFadeIn) 1.0)
  (bind _newtrack_1 (Timeline|FadeIn PlayFromStart)))

(event Custom|HudFadeOut
  ;[1 0.2974 0.5828] Actual HUD
  (Components|Timeline|SetPlayRate (Variables|Default|GetFadeIn) 1.0)
  (bind _newtrack_1 (Timeline|FadeIn ReverseFromEnd)))

(event Custom|HudIsToldPlayerDied
  ;[1 0.2974 0.5828] Actual HUD
  (Components|Timeline|SetPlayRate (Variables|Default|GetFadeIn) (Variables|Default|GetDeathPlayrate))
  (bind _newtrack_1 (Timeline|FadeIn ReverseFromEnd)))

(event EventDrawHUD
  (params (SizeX :type Integer) (SizeY :type Integer))
  ;[1 0.2974 0.5828] Actual HUD
  (Variables|Default|SetCurrentResolutionX SizeX)
  (Variables|Default|SetCurrentResolutionY SizeY)
  (Variables|Default|SetGlobalHUDScale (Math|Float|Clamp(Float) (/ (Math|Conversions|ToFloat(Integer) (Variables|Default|GetCurrentResolutionX)) 1.2e+03) 0.6 1.125))
  (bind _assolusplayercontroller_c (Utilities|Casting|CastToSolusPlayerController (Game|GetPlayerController 0))
    (:then
      _)
    (:CastFailed
      _))
  (if (Variables|/Game/Blueprints/Game/SolusPlayerController.SolusPlayerController_C|GetAllowInput _assolusplayercontroller_c)
    (Variables|Default|SetShowCrosshair true)
    (else
      (Variables|Default|SetShowCrosshair false)))
  (HUD|DrawRect (Math|Color|MakeColor 0.0 0.0 0.0 (stale Custom|HudFadeIn _newtrack_1)) 0.0 0.0 4096.0 4096.0)
  ;[0.363 1 0.4952] Crosshair
  (if (Variables|Default|GetShowCrosshair)
    (Class|HUD|DrawMaterialSimple "/Game/Player/HUD/Materials/MAT_Player_Crosshair.MAT_Player_Crosshair" (/ (Math|Conversions|ToFloat(Integer) (Variables|Default|GetCurrentResolutionX)) 2.01) (/ (Math|Conversions|ToFloat(Integer) (Variables|Default|GetCurrentResolutionY)) 2.01) 7.0 7.0 (Variables|Default|GetGlobalHUDScale) false)))

(event EventBeginPlay
  ;[1 0.2974 0.5828] Actual HUD
  (Components|Timeline|SetPlayRate (Variables|Default|GetFadeIn) 1.0)
  (bind _newtrack_1 (Timeline|FadeIn PlayFromStart)))

(fn ConstructionScript)