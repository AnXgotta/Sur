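; SolusPlayer is the player pawn, handling hand animation, footsteps, environment detection and swimming, and saving its spawn as the default checkpoint.
; A speed-scaled delay loop drops alternating footprint decals with sound, while Tick adjusts hand animation rate and depth-based cave smoke.
; A half-second loop sets Indoors using five upward traces above a height threshold.
; Water volumes trigger swimming, sinking, muffled audio, screen effects and repeating drowning feedback via DoOnce-gated timelines.
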(event Custom|IdleAnimation
  (bind _handanimation (Variables|SolusPlayer|GetHandAnimation))
  ;[1 1 1] Idle Animation hand
  (Components|Animation|SetAnimation _handanimation "/Game/Player/Character/Meshes/Anim_Player_Hand_Idle.Anim_Player_Hand_Idle")
  (Audio|Components|Audio|Play _handanimation true))

(event Custom|IndoorCheck
  ;[1 1 1] Indoor check
  (Utilities|FlowControl|Delay 0.5)
  (if (< (.Z (Math|Vector|BreakVector (Transformation|GetActorLocation (Game|Player|GetPlayerPawn 0)))) -512.0)
    (CallFunction|IndoorCheck)
    (else
      (bind _tracehitsomething (CallFunction|NearbyTraceCheck 0.0 0.0))
      (if _tracehitsomething
        (bind _tracehitsomething_2 (CallFunction|NearbyTraceCheck 2e+02 0.0))
        (if _tracehitsomething_2
          (bind _tracehitsomething_3 (CallFunction|NearbyTraceCheck -2e+02 0.0))
          (if _tracehitsomething_3
            (bind _tracehitsomething_4 (CallFunction|NearbyTraceCheck 0.0 2e+02))
            (if _tracehitsomething_4
              (bind _tracehitsomething_5 (CallFunction|NearbyTraceCheck 0.0 -2e+02))
              (if _tracehitsomething_5
                (Variables|Default|SetIndoors true)
                (else
                  (Variables|Default|SetIndoors false :!label _label)))
              (else
                (goto _label)))
            (else
              (goto _label)))
          (else
            (goto _label)))
        (else
          (goto _label)))
      (CallFunction|IndoorCheck))))

(event Custom|FootstepRestart
  (bind _returnvalue (Game|Player|GetPlayerPawn 0))
  (bind _soundfootsteps (Variables|SolusPlayer|GetSoundFootsteps))
  (bind _returnvalue_2 (Transformation|GetVelocity _returnvalue))
  (bind _returnvalue_3 (Transformation|GetActorLocation _returnvalue))
  (bind _returnvalue_4 (Transformation|GetActorRotation _returnvalue))
  (bind (_x _y _z) (Math|Vector|BreakVector _returnvalue_2))
  (bind _yaw (Class|KismetMathLibrary|BreakRot _returnvalue_4))
  (bind _returnvalue_5 (- _returnvalue_3 "0, 0,120.000000"))
  (bind _returnvalue_6 (Class|KismetMathLibrary|MakeRot 2.7e+02 _yaw 0.0))
  ;[1 1 1] Leaving Footsteps behind
  (Math|Float|CompareFloat (+ (Math|Float|Absolute(Float) _x) (Math|Float|Absolute(Float) _y)) 2e+01
    (:>
      (Math|Float|CompareFloat _z 0.0
        (:>
          (CallFunction|FootstepGoDirectlytoEnd :!label _label))
        (:==
          (Utilities|FlowControl|FlipFlop
            (:A
              (Rendering|Decal|SpawnDecalatLocation "/Game/Player/FX/Materials/MAT_Player_Footsteps01.MAT_Player_Footsteps01" "64.000000,64.000000,32.000000" _returnvalue_5 _returnvalue_6 16.0))
            (:B
              (Rendering|Decal|SpawnDecalatLocation "/Game/Player/FX/Materials/MAT_Player_Footsteps02.MAT_Player_Footsteps02" "64.000000,64.000000,32.000000" _returnvalue_5 _returnvalue_6 16.0)))
          (Audio|Components|Audio|SetSound _soundfootsteps "/Game/Sounds/Player/Gameplay/Cue/SO_PlayerSound_Footstep_Cue.SO_PlayerSound_Footstep_Cue")
          (Audio|Components|Audio|Play _soundfootsteps 0.0)
          (Utilities|FlowControl|RetriggerableDelay (/ (Math|Float|Clamp(Float) (Class|KismetMathLibrary|MapRange (Variables|/Script/Engine.CharacterMovementComponent|GetMaxWalkSpeed (Variables|Character|GetCharacterMovement)) 4e+02 2e+02 1.0 2.0) 1.0 2.0) 4.0) :!label _label_2)
          (CallFunction|FootstepRestart))
        (:<
          (goto _label_2))))
    (:==
      (goto _label))
    (:<
      (goto _label))))

(event Custom|FootstepGoDirectlyToEnd
  ;[1 1 1] Leaving Footsteps behind
  (Utilities|FlowControl|RetriggerableDelay (/ (Math|Float|Clamp(Float) (Class|KismetMathLibrary|MapRange (Variables|/Script/Engine.CharacterMovementComponent|GetMaxWalkSpeed (Variables|Character|GetCharacterMovement)) 4e+02 2e+02 1.0 2.0) 1.0 2.0) 4.0))
  (CallFunction|FootstepRestart))

(event Custom|RestartDrown
  (bind _soundplayer (Variables|SolusPlayer|GetSoundPlayer))
  ;[1 1 1] Drowning
  (if (Variables|/Script/Engine.PhysicsVolume|GetbWaterVolume (Class|MovementComponent|GetPhysicsVolume (Variables|Character|GetCharacterMovement)))
    (if (not (<= (Variables|Default|GetHealthPlayer) 0))
      (Audio|Components|Audio|SetSound _soundplayer "/Game/Sounds/Player/Gameplay/Cue/SO_PlayerSound_Drown_Cue.SO_PlayerSound_Drown_Cue")
      (Audio|Components|Audio|Play _soundplayer 0.0)
      (AddComponent|AddParticleSystemComponent true (Transformation|GetActorTransform (Game|Player|GetPlayerPawn 0)))
      (Utilities|FlowControl|Delay 2.0)
      (CallFunction|RestartDrown))))

(event EventTick
  (params (DeltaSeconds :type Float%20%28single-precision%29))
  (bind _soundplayer (Variables|SolusPlayer|GetSoundPlayer))
  ;[0.3118 0.5924 1] Continous Update
  (Utilities|FlowControl|Sequence
    (:then_1
      ;[1 1 1] Cave Smoke and idle anim speed
      (CallFunction|CaveSmokeEnabler)
      (CallFunction|RunningAffectsIddleAnimation))
    (:then_4
      ;[1 1 1] set water behaviour
      (if (Variables|/Script/Engine.PhysicsVolume|GetbWaterVolume (Class|MovementComponent|GetPhysicsVolume (Variables|Character|GetCharacterMovement)))
        (Utilities|FlowControl|DoOnce false :!label _label
          (:Completed
            (Utilities|FlowControl|Sequence
              (:then_0
                (Pawn|Components|CharacterMovement|SetMovementMode (Variables|Character|GetCharacterMovement) "MOVE_Swimming")
                (Audio|PushSoundMixModifier "/Game/Sounds/Classes/SolusUnderwater.SolusUnderwater")
                (Utilities|FlowControl|Sequence
                  (:then_0
                    (bind _curve (Timeline|Timeline_1 Play)
                      (:Update
                        (Variables|/Script/Engine.MovementComponent|SetVelocity (Variables|Character|GetCharacterMovement) (Math|Vector|Lerp(Vector) (Transformation|GetVelocity (Game|Player|GetPlayerPawn 0)) "0,0.000000,-50.000000" _curve)))))
                  (:then_1
                    ;[1 1 1] Drowning
                    (Utilities|FlowControl|RetriggerableDelay 5.0)
                    (if (Variables|/Script/Engine.PhysicsVolume|GetbWaterVolume (Class|MovementComponent|GetPhysicsVolume (Variables|Character|GetCharacterMovement)))
                      (if (not (<= (Variables|Default|GetHealthPlayer) 0))
                        (Audio|Components|Audio|SetSound _soundplayer "/Game/Sounds/Player/Gameplay/Cue/SO_PlayerSound_Drown_Cue.SO_PlayerSound_Drown_Cue")
                        (Audio|Components|Audio|Play _soundplayer 0.0)
                        (AddComponent|AddParticleSystemComponent true (Transformation|GetActorTransform (Game|Player|GetPlayerPawn 0)))
                        (Utilities|FlowControl|Delay 2.0)
                        (CallFunction|RestartDrown))))))
              (:then_1
                (goto _label_2 Reset))
              (:then_2
                (bind _fadewatereffect (Timeline|Timeline_2 Play)
                  (:Update
                    (Rendering|Material|SetScalarParameterValue "/Game/Player/PostProcess/Materials/SolusPostProcessCollection.SolusPostProcessCollection" "DrownState" _fadewatereffect :!class /Script/Engine.KismetMaterialLibrary)))))))
        (else
          (Utilities|FlowControl|DoOnce false :!label _label_2
            (:Completed
              (Utilities|FlowControl|Sequence
                (:then_0
                  (goto _label Reset))
                (:then_1
                  (Timeline|Timeline_1 Stop))
                (:then_2
                  (Class|GameplayStatics|ClearSoundMixModifiers)
                  (Timeline|Timeline_2 Reverse))))))))))

(event EventBeginPlay
  (bind _handanimation (Variables|SolusPlayer|GetHandAnimation))
  ;[0.3363 0.6591 1] Start Game
  (Utilities|FlowControl|Sequence
    (:then_0
      ;[1 1 1] Idle Animation hand
      (Components|Animation|SetAnimation _handanimation "/Game/Player/Character/Meshes/Anim_Player_Hand_Idle.Anim_Player_Hand_Idle")
      (Audio|Components|Audio|Play _handanimation true))
    (:then_1
      ;[1 1 1] Leaving Footsteps behind
      (Utilities|FlowControl|RetriggerableDelay (/ (Math|Float|Clamp(Float) (Class|KismetMathLibrary|MapRange (Variables|/Script/Engine.CharacterMovementComponent|GetMaxWalkSpeed (Variables|Character|GetCharacterMovement)) 4e+02 2e+02 1.0 2.0) 1.0 2.0) 4.0))
      (CallFunction|FootstepRestart))
    (:then_2
      ;[1 1 1] Start Indoor and Outdoor check
      (CallFunction|IndoorCheck))
    (:then_4
      ;[1 1 1] store start loc as default checkpoint
      (bind _assolusgamestate_c (Utilities|Casting|CastToSolusGameState (Game|GetGameState)))
      (Variables|/Game/Blueprints/Game/SolusGameState.SolusGameState_C|SetPlayerCheckPointTransform _assolusgamestate_c (Transformation|GetActorTransform (Game|Player|GetPlayerPawn 0))))))

(fn ConstructionScript
  (bind _assolusgamestate_c (Utilities|Casting|CastToSolusGameState (Game|GetGameState))
    (:then
      _)
    (:CastFailed
      _))
  (Variables|Default|SetHealthPlayer (Variables|/Game/Blueprints/Game/SolusGameState.SolusGameState_C|GetPlayerHealth _assolusgamestate_c)))

(fn NearbyTraceCheck
  (params (XOffset :type Float%20%28single-precision%29) (YOffset :type Float%20%28single-precision%29))
  (bind _returnvalue (Game|Player|GetPlayerPawn 0))
  (bind _returnvalue_2 (Transformation|GetActorLocation _returnvalue))
  (bind (_x _y _z) (Math|Vector|BreakVector _returnvalue_2))
  (bind _returnvalue_3 (+ _y YOffset))
  (bind _returnvalue_4 (+ _x XOffset))
  (bind _returnvalue_5 (Collision|LineTraceForObjects (Math|Vector|MakeVector _returnvalue_4 _returnvalue_3 _z) (Math|Vector|MakeVector _returnvalue_4 _returnvalue_3 (+ _z 5e+03)) (Utilities|Array|MakeArray (Variables|Default|GetObjectToTrace)) false 0 "None"))
  (return _returnvalue_5))

(fn CaveSmokeEnabler
  (bind _returnvalue (Game|Player|GetPlayerPawn 0))
  (bind _cavesmoke (Variables|SolusPlayer|GetCaveSmoke))
  (bind _returnvalue_2 (Transformation|GetActorLocation _returnvalue))
  (bind _z (Math|Vector|BreakVector _returnvalue_2))
  (if (< _z -768.0)
    (Components|Activation|Activate _cavesmoke false)
    (Effects|Components|ParticleSystem|SetFloatParameter (Variables|SolusPlayer|GetCaveSmoke) "rate" (Math|Float|Clamp(Float) (Class|KismetMathLibrary|MapRange _z -768.0 -1536.0 0.0 1.0)))
    (else
      (Components|Activation|Deactivate _cavesmoke))))

(fn RunningAffectsIddleAnimation
  (bind _self self)
  (bind _returnvalue (Transformation|GetVelocity _self))
  (bind (_x _y) (Math|Vector|BreakVector _returnvalue))
  (Components|Timeline|SetPlayRate (Variables|SolusPlayer|GetHandAnimation) (Math|Float|Clamp(Float) (* (+ (Math|Float|Absolute(Float) _x) (Math|Float|Absolute(Float) _y)) 0.01) 1.0 4.0)))