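; Player controller for the Solus player, handling first-person input, debug cheats and death camera animations.
; Gated input drives look, movement, swimming in water volumes, a PlayerSpeed toggle, and jumps with velocity boost, sound and timed DoOnce lockout.
; CameraDeath and CameraDrowning save control rotation, animate it through timelines, then reset roll.
; Flag-gated debug keys toggle slow motion, fast walk, fly and high-speed noclip.
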(event Custom|SolusPlayerForceJump
  (bind _returnvalue (Game|Player|GetPlayerPawn 0))
  (bind _returnvalue_2 (Game|Player|GetPlayerPawn 0))
  (bind _soundplayer (Variables|SolusPlayerController|GetSoundPlayer))
  (bind _returnvalue_3 (Pawn|GetMovementComponent _returnvalue))
  ;[1 10 0] FPS CORE CONTROLS
  (if (Variables|Default|GetAllowInput)
    (if (not (Variables|/Script/Engine.PhysicsVolume|GetbWaterVolume (Class|MovementComponent|GetPhysicsVolume (Pawn|GetMovementComponent _returnvalue_2))))
      (bind _assolusplayer_c (Utilities|Casting|CastToSolusPlayer _returnvalue_2))
      (Variables|/Game/Blueprints/Game/SolusPlayer.SolusPlayer_C|SetPlayersLocationTopofFall _assolusplayer_c (Transformation|GetActorLocation _returnvalue_2))
      (Utilities|FlowControl|Sequence
        (:then_0
          (Utilities|FlowControl|DoOnce false :!label _label
            (:Completed
              (bind _assolusplayer_c_2 (Utilities|Casting|CastToSolusPlayer (Game|Player|GetPlayerPawn 0)))
              (Character|Jump _assolusplayer_c_2)
              (Variables|/Script/Engine.MovementComponent|SetVelocity _returnvalue_3 (* (Variables|/Script/Engine.MovementComponent|GetVelocity _returnvalue_3) 1.2))
              (Audio|Components|Audio|SetSound _soundplayer "/Game/Sounds/Player/Gameplay/Cue/SO_PlayerSound_Jump_Cue.SO_PlayerSound_Jump_Cue")
              (Audio|Components|Audio|Play _soundplayer 0.0))))
        (:then_1
          (Utilities|FlowControl|Delay 1.0)
          (goto _label Reset))))))

(event Custom|ResetRoll
  (bind _rotationbeforedeath (Variables|Default|GetRotationBeforeDeath))
  (bind (_pitch _yaw) (Class|KismetMathLibrary|BreakRot _rotationbeforedeath))
  ;[1 1 1] camera animation
  ;;[1 1 1] Reset Roll after death
  (Utilities|FlowControl|RetriggerableDelay 0.4)
  (Pawn|SetControlRotation (Class|KismetMathLibrary|MakeRot _pitch _yaw 0.0)))

(event Custom|CameraDeath
  ;[1 1 1] camera animation
  ;;[1 1 1] General death
  (Utilities|FlowControl|Sequence
    (:then_1
      (Variables|Default|SetRotationBeforeDeath (Pawn|GetControlRotation :!class /Script/Engine.Controller))
      (bind (_direction _general_pitch _general_roll) (Timeline|Timeline_4 PlayFromStart)
        (:Update
          (Pawn|SetControlRotation (Class|KismetMathLibrary|MakeRot (.Pitch (Class|KismetMathLibrary|BreakRot (Math|Rotator|MakeRotationfromAxes (Math|Vector|MakeVector (.X (Math|Vector|BreakVector (.X (Math|Rotator|BreakRotIntoAxes (Variables|Default|GetRotationBeforeDeath))))) (.Y (Math|Vector|BreakVector (.X (Math|Rotator|BreakRotIntoAxes (Variables|Default|GetRotationBeforeDeath))))) (+ _general_pitch (.Z (Math|Vector|BreakVector (.X (Math|Rotator|BreakRotIntoAxes (Variables|Default|GetRotationBeforeDeath))))))) (.Y (Math|Rotator|BreakRotIntoAxes (Variables|Default|GetRotationBeforeDeath))) (.Z (Math|Rotator|BreakRotIntoAxes (Variables|Default|GetRotationBeforeDeath)))))) (.Yaw (Class|KismetMathLibrary|BreakRot (Math|Rotator|MakeRotationfromAxes (Math|Vector|MakeVector (.X (Math|Vector|BreakVector (.X (Math|Rotator|BreakRotIntoAxes (Variables|Default|GetRotationBeforeDeath))))) (.Y (Math|Vector|BreakVector (.X (Math|Rotator|BreakRotIntoAxes (Variables|Default|GetRotationBeforeDeath))))) (+ _general_pitch (.Z (Math|Vector|BreakVector (.X (Math|Rotator|BreakRotIntoAxes (Variables|Default|GetRotationBeforeDeath))))))) (.Y (Math|Rotator|BreakRotIntoAxes (Variables|Default|GetRotationBeforeDeath))) (.Z (Math|Rotator|BreakRotIntoAxes (Variables|Default|GetRotationBeforeDeath)))))) (+ (* _general_roll 25.0) (.Roll (Class|KismetMathLibrary|BreakRot (Variables|Default|GetRotationBeforeDeath)))))))
        (:Finished
          (CallFunction|ResetRoll))))))

(event Custom|CameraDrowning
  ;[1 1 1] camera animation
  ;;[1 1 1] Drowning
  (Variables|Default|SetRotationBeforeDeath (Pawn|GetControlRotation :!class /Script/Engine.Controller))
  (Utilities|FlowControl|Sequence
    (:then_0
      (bind _drowning_lookingup (Timeline|LookingUpDrowning PlayFromStart)
        (:Update
          (Pawn|SetControlRotation (Class|KismetMathLibrary|MakeRot (.Pitch (Class|KismetMathLibrary|BreakRot (Math|Rotator|MakeRotationfromAxes (Math|Vector|MakeVector (.X (Math|Vector|BreakVector (.X (Math|Rotator|BreakRotIntoAxes (Variables|Default|GetRotationBeforeDeath))))) (.Y (Math|Vector|BreakVector (.X (Math|Rotator|BreakRotIntoAxes (Variables|Default|GetRotationBeforeDeath))))) (+ _drowning_lookingup (.Z (Math|Vector|BreakVector (.X (Math|Rotator|BreakRotIntoAxes (Variables|Default|GetRotationBeforeDeath))))))) (.Y (Math|Rotator|BreakRotIntoAxes (Variables|Default|GetRotationBeforeDeath))) (.Z (Math|Rotator|BreakRotIntoAxes (Variables|Default|GetRotationBeforeDeath)))))) (+ (.Yaw (Class|KismetMathLibrary|BreakRot (Variables|Default|GetRotationBeforeDeath))) (* 3.0 (stale _drowning_yawright))) (+ (stale _drowning_roll) (.Roll (Class|KismetMathLibrary|BreakRot (Variables|Default|GetRotationBeforeDeath)))))))
        (:Finished
          (CallFunction|ResetRoll))))
    (:then_1
      (bind (_direction _drowning_yawright _drowning_roll) (Timeline|DrowningStruggleRight PlayFromStart)))))

(event Input|ActionEvents|InputActionSolusSprint
  ;[1 10 0] FPS CORE CONTROLS
  (:Pressed
    (if (Variables|Default|GetAllowInput)
      (Utilities|FlowControl|FlipFlop
        (:A
          (Variables|Default|SetPlayerSpeed 2e+02))
        (:B
          (Variables|Default|SetPlayerSpeed 4e+02))))))

(event Input|ActionEvents|InputActionJump
  (bind _returnvalue (Game|Player|GetPlayerPawn 0))
  (bind _returnvalue_2 (Game|Player|GetPlayerPawn 0))
  (bind _soundplayer (Variables|SolusPlayerController|GetSoundPlayer))
  (bind _returnvalue_3 (Pawn|GetMovementComponent _returnvalue))
  ;[1 10 0] FPS CORE CONTROLS
  (:Pressed
    (if (Variables|Default|GetAllowInput)
      (if (not (Variables|/Script/Engine.PhysicsVolume|GetbWaterVolume (Class|MovementComponent|GetPhysicsVolume (Pawn|GetMovementComponent _returnvalue_2))))
        (bind _assolusplayer_c (Utilities|Casting|CastToSolusPlayer _returnvalue_2))
        (Variables|/Game/Blueprints/Game/SolusPlayer.SolusPlayer_C|SetPlayersLocationTopofFall _assolusplayer_c (Transformation|GetActorLocation _returnvalue_2))
        (Utilities|FlowControl|Sequence
          (:then_0
            (Utilities|FlowControl|DoOnce false :!label _label
              (:Completed
                (bind _assolusplayer_c_2 (Utilities|Casting|CastToSolusPlayer (Game|Player|GetPlayerPawn 0)))
                (Character|Jump _assolusplayer_c_2)
                (Variables|/Script/Engine.MovementComponent|SetVelocity _returnvalue_3 (* (Variables|/Script/Engine.MovementComponent|GetVelocity _returnvalue_3) 1.2))
                (Audio|Components|Audio|SetSound _soundplayer "/Game/Sounds/Player/Gameplay/Cue/SO_PlayerSound_Jump_Cue.SO_PlayerSound_Jump_Cue")
                (Audio|Components|Audio|Play _soundplayer 0.0))))
          (:then_1
            (Utilities|FlowControl|Delay 1.0)
            (goto _label Reset)))))))

(event Input|AxisEvents|InputAxisTurn
  (params (AxisValue :type Float%20%28single-precision%29))
  ;[1 10 0] FPS CORE CONTROLS
  (if (Variables|Default|GetAllowInput)
    (Class|PlayerController|AddYawInput AxisValue)))

(event Input|AxisEvents|InputAxisLookUp
  (params (AxisValue :type Float%20%28single-precision%29))
  ;[1 10 0] FPS CORE CONTROLS
  (if (Variables|Default|GetAllowInput)
    (Class|PlayerController|AddPitchInput AxisValue)))

(event Input|AxisEvents|InputAxisMoveForward
  (params (AxisValue :type Float%20%28single-precision%29))
  ;[1 10 0] FPS CORE CONTROLS
  (if (Variables|Default|GetAllowInput)
    (Pawn|Input|AddMovementInput (Game|Player|GetPlayerPawn 0) (Math|Vector|GetForwardVector (Pawn|GetControlRotation :!class /Script/Engine.Controller)) AxisValue)))

(event Input|AxisEvents|InputAxisMoveRight
  (params (AxisValue :type Float%20%28single-precision%29))
  ;[1 10 0] FPS CORE CONTROLS
  (if (Variables|Default|GetAllowInput)
    (Pawn|Input|AddMovementInput (Game|Player|GetPlayerPawn 0) (Math|Vector|GetRightVector (Pawn|GetControlRotation :!class /Script/Engine.Controller)) AxisValue)))

(event Input|AxisEvents|InputAxisMoveUp
  (params (AxisValue :type Float%20%28single-precision%29))
  ;[1 10 0] FPS CORE CONTROLS
  (if (Variables|Default|GetAllowInput)
    (if (Variables|/Script/Engine.PhysicsVolume|GetbWaterVolume (Class|MovementComponent|GetPhysicsVolume (Pawn|GetMovementComponent (Game|Player|GetPlayerPawn 0))))
      (Pawn|Input|AddMovementInput (Game|Player|GetPlayerPawn 0) (Math|Vector|GetUpVector (Pawn|GetControlRotation :!class /Script/Engine.Controller)) AxisValue))))

(event Input|KeyboardEvents|P
  ;[9.332 0.5628 10] DEBUG CONTROLS
  (:Pressed
    (if (Variables|Default|GetAllowDebugControls)
      (Utilities|FlowControl|FlipFlop
        (:A
          (Development|ExecuteConsoleCommand "slomo 4")
          (Development|ExecuteConsoleCommand "ghost")
          (Development|PrintString "no clip super speed on"))
        (:B
          (Development|ExecuteConsoleCommand "slomo 1")
          (Development|ExecuteConsoleCommand "walk")
          (Development|PrintString "no clip super speed off"))))))

(event Input|KeyboardEvents|I
  ;[9.332 0.5628 10] DEBUG CONTROLS
  (:Pressed
    (if (Variables|Default|GetAllowDebugControls)
      (Utilities|FlowControl|FlipFlop
        (:A
          (Variables|Default|SetPlayerSpeed 1e+03)
          (Development|PrintString "fast walk speed"))
        (:B
          (Variables|Default|SetPlayerSpeed 4e+02)
          (Development|PrintString "normal walk speed"))))))

(event Input|KeyboardEvents|O
  ;[9.332 0.5628 10] DEBUG CONTROLS
  (:Pressed
    (if (Variables|Default|GetAllowDebugControls)
      (Utilities|FlowControl|FlipFlop
        (:A
          (Development|ExecuteConsoleCommand "fly")
          (Development|PrintString "fly"))
        (:B
          (Development|ExecuteConsoleCommand "walk")
          (Development|PrintString "walk"))))))

(event Input|KeyboardEvents|U
  ;[9.332 0.5628 10] DEBUG CONTROLS
  (:Pressed
    (if (Variables|Default|GetAllowDebugControls)
      _)))

(event Input|KeyboardEvents|Y
  ;[9.332 0.5628 10] DEBUG CONTROLS
  (:Pressed
    (if (Variables|Default|GetAllowDebugControls)
      (Utilities|FlowControl|FlipFlop
        (:A
          (Development|ExecuteConsoleCommand "slomo 0.1")
          (Development|PrintString "slomo on"))
        (:B
          (Development|ExecuteConsoleCommand "slomo 1")
          (Development|PrintString "slomo off"))))))

(fn ConstructionScript)