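; Test HUD that draws the player's inventory as plain on-screen text while ShowInventory is true.
; DrawHUD draws an INVENTORY title, then reads the inventory from the owning BP_SurCharacter.
; Each non-empty slot's item name, suffixed with its display index, prints on its own row scaled to screen height.
; The row index increments per item and resets to a fixed starting row after the loop.
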(event EventDrawHUD
  (params (SizeX :type Integer) (SizeY :type Integer))
  (Variables|Default|SetScreenDimensions (Math|Vector2D|MakeVector2D (Math|Conversions|ToFloat(Integer) SizeX) (Math|Conversions|ToFloat(Integer) SizeY)))
  (Utilities|FlowControl|Sequence
    (:then_0
      (if (Variables|Default|GetShowInventory)
        (Utilities|FlowControl|Sequence
          (:then_0
            (HUD|DrawText "INVENTORY" "(R=1.000000,G=0.000000,B=0.862927,A=1.000000)" (/ (.X (Math|Vector2D|BreakVector2D (Variables|Default|GetScreenDimensions))) 2.0) (* 0 (/ (.Y (Math|Vector2D|BreakVector2D (Variables|Default|GetScreenDimensions))) 4e+01)) 0 3.0 false))
          (:then_1
            (bind _asbp_surcharacter_c (Utilities|Casting|CastToBP_SurCharacter (Class|HUD|GetOwningPawn)))
            (bind _returnvalue (Class|SurCharacter|GetInventory _asbp_surcharacter_c))
            (for _array_element _returnvalue
              (bind _returnvalue_2 (Class|SurInventorySlot|IsSlotEmpty _array_element))
              (if (not _returnvalue_2)
                (bind _returnvalue_3 (Class|SurInventorySlot|GetItemName _array_element))
                (HUD|DrawText (Utilities|String|Append (Utilities|String|ToString(Name) _returnvalue_3) (Utilities|String|ToString(Integer) (Variables|Default|GetInventoryDisplayIndex))) "(R=0.113357,G=1.000000,B=0.000000,A=1.000000)" (/ (.X (Math|Vector2D|BreakVector2D (Variables|Default|GetScreenDimensions))) 2.0) (* (Variables|Default|GetInventoryDisplayIndex) (/ (.Y (Math|Vector2D|BreakVector2D (Variables|Default|GetScreenDimensions))) 4e+01)) 0 2.0 false)
                (Variables|Default|SetInventoryDisplayIndex (+ (Variables|Default|GetInventoryDisplayIndex) 1))))
            (Variables|Default|SetInventoryDisplayIndex 5)))))))

(fn ConstructionScript)