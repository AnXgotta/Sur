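; BP_HUD_Test is a test HUD Blueprint with helpers for placing and sizing textures as fractions of the screen.
; DrawScaledTexture passes position and size through AdjustForScreenRes, which multiplies by ScreenDimensions, then draws opaque.
; GetScreenBasedValues does the same conversion on vector inputs.
; DrawHUD is empty, ScreenDimensions is never set here, and the ideal-resolution input and scale outputs are unused placeholders.
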(event EventDrawHUD
  (params (SizeX :type Integer) (SizeY :type Integer)))

(fn ConstructionScript)

(fn AdjustforScreenRes
  (params (TexturePosX :type Float%20%28single-precision%29) (TexturePosY :type Float%20%28single-precision%29) (TextureWidth :type Float%20%28single-precision%29) (TextureHeight :type Float%20%28single-precision%29) (IdealScreenResolution :type Vector%202D%20Structure))
  (bind _screendimensions (Variables|Default|GetScreenDimensions))
  (bind (_x _y) (Math|Vector2D|BreakVector2D _screendimensions))
  (return (* TexturePosX _x) (* TexturePosY _y) (* TextureWidth _x) (* TextureHeight _y) 0.0 0.0))

(fn DrawScaledTexture
  (params (XPos :type Float%20%28single-precision%29) (YPos :type Float%20%28single-precision%29) (Width :type Float%20%28single-precision%29) (Height :type Float%20%28single-precision%29) (IdealScreenSize :type Vector%202D%20Structure) (Texture :type Texture%202D%20Object%20Reference))
  (bind (_textureposxout _textureposyout _texturewidthout _textureheightout) (CallFunction|AdjustforScreenRes XPos YPos Width Height IdealScreenSize))
  (Canvas|DrawTexture Texture _textureposxout _textureposyout _texturewidthout _textureheightout 0.0 1.0 1.0 1.0 "(R=1.000000,G=1.000000,B=1.000000,A=1.000000)" "BLEND_Opaque"))

(fn GetScreenBasedValues
  (params (PositionPercentTotal :type Vector%202D%20Structure) (SizePercentTotal :type Vector%202D%20Structure))
  (bind (_x _y) (Math|Vector2D|BreakVector2D PositionPercentTotal))
  (bind (_x_2 _y_2) (Math|Vector2D|BreakVector2D SizePercentTotal))
  (bind _screendimensions (Variables|Default|GetScreenDimensions))
  (bind (_x_3 _y_3) (Math|Vector2D|BreakVector2D _screendimensions))
  (return (Math|Vector2D|MakeVector2D (* _x_3 _x) (* _y_3 _y)) (Math|Vector2D|MakeVector2D (* _x_3 _x_2) (* _y_3 _y_2))))